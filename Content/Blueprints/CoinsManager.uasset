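; CoinsManager is an actor that keeps the coin total and displays it alongside a running game timer on text render components.
; AddCoins and SubstractCoins adjust CurrentCoins and refresh the coin text, with no bounds checks.
; Tick rebuilds the timer text from time since the actor's creation as unpadded hours, minutes, seconds and milliseconds; InitTime is recorded but unused here.
; The construction script fills both texts initially.
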(event `self.ReceiveBeginPlay`
  (set `self.InitTime` (`KismetMathLibrary.Now`)))

(event `self.ReceiveTick`
  (params (DeltaSeconds :type "Float (single-precision)"))
  (`self.UpdateTimeText`))

(fn `AddCoins`
  (params (CoindAddition :type Integer))
  (bind _output_get (set `self.CurrentCoins` (+ (`self.CurrentCoins`) CoindAddition)))
  (`TextRenderComponent.K2_SetText` (`TextRenderActor.TextRender` (`self.CoinsText`)) (`KismetTextLibrary.Conv_IntToText` _output_get)))

(fn `SubstractCoins`
  (params (CoindSubstraction :type Integer))
  (bind _output_get (set `self.CurrentCoins` (- (`self.CurrentCoins`) CoindSubstraction)))
  (`TextRenderComponent.K2_SetText` (`TextRenderActor.TextRender` (`self.CoinsText`)) (`KismetTextLibrary.Conv_IntToText` _output_get)))

(fn `UpdateTimeText`
  (bind (_days _hours _minutes _seconds _milliseconds) (`KismetMathLibrary.BreakTimespan` (`KismetMathLibrary.FromSeconds` (`self.GetGameTimeSinceCreation`))))
  (`TextRenderComponent.K2_SetText` (`TextRenderActor.TextRender` (`self.TimeText`)) (`KismetTextLibrary.Conv_StringToText` (`KismetStringLibrary.Concat_StrStr` (`KismetStringLibrary.Conv_IntToString` _hours) ":" (`KismetStringLibrary.Conv_IntToString` _minutes) ":" (`KismetStringLibrary.Conv_IntToString` _seconds) ":" (`KismetStringLibrary.Conv_IntToString` _milliseconds)))))

(fn `UserConstructionScript`
  (`self.UpdateTimeText`)
  (`self.AddCoins` 0))