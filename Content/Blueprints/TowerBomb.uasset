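; Bomb tower for a tower defense game that turns toward the first enemy in its radius and fires projectiles on a cooldown.
; Launch speed is computed from target distance and the head's height and fixed pitch.
; Clicking toggles camera-facing text options to repair, upgrade or sell through ScoreController coins; upgrades improve health, damage and fire rate and tint the dynamic material.
; Selling or fatal damage replaces the tower with a TowerSpawnPoint.
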(event `self.ReceiveBeginPlay`
  (bind _lifetext (`self.LifeText`))
  (set `self.CurrentHealthPoints` (`self.MaxHealthPoints`))
  (`KismetArrayLibrary.Array_Append` (`PrimitiveComponent.GetOverlappingActors` (`self.ShootingRadius`) "/Game/Blueprints/Enemy.Enemy_C") (`self.PotentialTargets`))
  (bind _outactors (`GameplayStatics.GetAllActorsOfClass` "/Script/Engine.CameraActor"))
  (for _array_element _outactors
    (if (`KismetStringLibrary.EqualEqual_StrStr` (`KismetStringLibrary.Conv_ObjectToString` _array_element) "PlayerCamera")
      (bind _output_get (set `self.CameraActor` _array_element))))
  (bind _output_get_2 (set `self.LookAtCameraRotation` (`KismetMathLibrary.FindLookAtRotation` (`SceneComponent.K2_GetComponentLocation` _lifetext) (`self.K2_GetActorLocation` _output_get))))
  (`SceneComponent.K2_SetWorldRotation` _lifetext _output_get_2 false false)
  (`SceneComponent.K2_SetWorldRotation` (`self.RepairText`) _output_get_2 false false)
  (`SceneComponent.K2_SetWorldRotation` (`self.UpgradeText`) _output_get_2 false false)
  (`SceneComponent.K2_SetWorldRotation` (`self.SellText`) _output_get_2 false false)
  (`self.SetLifeText`))

(event `self.ShootingRadius.OnComponentEndOverlap`
  (params (OverlappedComponent :type "PrimitiveComponent Object Reference") (OtherActor :type "Actor Object Reference") (OtherComp :type "PrimitiveComponent Object Reference") (OtherBodyIndex :type Integer))
  (`KismetArrayLibrary.Array_RemoveItem` (`self.PotentialTargets`) OtherActor))

(event `self.ReceiveTick`
  (params (DeltaSeconds :type "Float (single-precision)"))
  (bind _towerhead (`self.TowerHead`))
  (bind _lifetext (`self.LifeText`))
  (bind _shotspawn (`self.ShotSpawn`))
  (`SceneComponent.K2_SetWorldRotation` _lifetext (`KismetMathLibrary.FindLookAtRotation` (`SceneComponent.K2_GetComponentLocation` _lifetext) (`self.K2_GetActorLocation` (`self.CameraActor`))) false false)
  (`SceneComponent.K2_SetWorldRotation` (`self.UpgradeText`) (`KismetMathLibrary.FindLookAtRotation` (`SceneComponent.K2_GetComponentLocation` _lifetext) (`self.K2_GetActorLocation` (`self.CameraActor`))) false false)
  (`SceneComponent.K2_SetWorldRotation` (`self.SellText`) (`KismetMathLibrary.FindLookAtRotation` (`SceneComponent.K2_GetComponentLocation` _lifetext) (`self.K2_GetActorLocation` (`self.CameraActor`))) false false)
  (`SceneComponent.K2_SetWorldRotation` (`self.RepairText`) (`KismetMathLibrary.FindLookAtRotation` (`SceneComponent.K2_GetComponentLocation` _lifetext) (`self.K2_GetActorLocation` (`self.CameraActor`))) false false)
  (if (> (`KismetArrayLibrary.Array_Length` (`self.PotentialTargets`)) 0)
    (`SceneComponent.K2_SetWorldRotation` _towerhead (`KismetMathLibrary.MakeRotator` 0.0 (.pitch (`SceneComponent.K2_GetComponentRotation` (`self.TowerHead`))) (.yaw (`KismetMathLibrary.FindLookAtRotation` (`SceneComponent.K2_GetComponentLocation` _towerhead) (`self.K2_GetActorLocation` (`|GetArrayItem` (`self.PotentialTargets`)))))) false false)
    (if (>= (- (`self.GetGameTimeSinceCreation`) (`self.TimeWhenLastShot`)) (`self.ShotCooldown`))
      (bind _initialspeed (`self.GetProjectileSpeed` (`self.K2_GetActorLocation` (`|GetArrayItem` (`self.PotentialTargets`)))))
      (`|SpawnActorFromClass` "/Game/Blueprints/Shot.Shot_C" (`KismetMathLibrary.MakeTransform` (`SceneComponent.K2_GetComponentLocation` _shotspawn) (`SceneComponent.K2_GetComponentRotation` _shotspawn)) "AlwaysSpawn" "OverrideRootScale" null (+ (`self.BombDamage`) (* (`self.PerLevelDamageIncrement`) (`self.Level`))) _initialspeed (+ (`self.LevelScaleIncrement`) (`self.BombScale`)) null)
      (set `self.TimeWhenLastShot` (`self.GetGameTimeSinceCreation`)))))

(event `self.ShootingRadius.OnComponentBeginOverlap`
  (params (OverlappedComponent :type "PrimitiveComponent Object Reference") (OtherActor :type "Actor Object Reference") (OtherComp :type "PrimitiveComponent Object Reference") (OtherBodyIndex :type Integer) (bFromSweep :type Boolean) (SweepResult :type "HitResult Structure (by ref)"))
  (if (`ActorComponent.ComponentHasTag` OtherComp "Enemy")
    (`KismetArrayLibrary.Array_Add` (`self.PotentialTargets`) OtherActor)))

(event `self.FullTowerClickListener.OnClicked`
  (params (TouchedComponent :type "PrimitiveComponent Object Reference") (ButtonPressed :type "Key Structure"))
  (bind _selltext (`self.SellText`))
  (bind _upgradetext (`self.UpgradeText`))
  (bind _repairtext (`self.RepairText`))
  (bind _returnvalue (`SceneComponent.IsVisible` _upgradetext))
  ;[1 1 1] OnTowerClicked
  (set `self.SelectionTime` (`self.GetGameTimeSinceCreation`))
  (`SceneComponent.SetVisibility` _repairtext (!= (`SceneComponent.IsVisible` _repairtext) true) false)
  (`SceneComponent.SetVisibility` _upgradetext (!= _returnvalue true) false)
  (`SceneComponent.SetVisibility` _selltext (!= (`SceneComponent.IsVisible` _selltext) true) false)
  (`self.SetTowerHover` _returnvalue))

(event `self.ClickListenerRepairText.OnClicked`
  (params (TouchedComponent :type "PrimitiveComponent Object Reference") (ButtonPressed :type "Key Structure"))
  ;[1 1 1] OnUpgrade/Repair/SellClicked
  (if (`SceneComponent.IsVisible` (`|GetArrayItem` (`SceneComponent.GetParentComponents` TouchedComponent)))
    (if (and (>= (`/Game/Blueprints/CoinsManager.CurrentCoins` (`self.ScoreController`)) (`self.RepairPrice`)) (!= (`self.CurrentHealthPoints`) (`self.MaxHealthPoints`)))
      (set `self.CurrentHealthPoints` (`self.MaxHealthPoints`))
      (`self.SetLifeText`)
      (`/Game/Blueprints/CoinsManager.SubstractCoins` (`self.ScoreController`) (`self.RepairPrice`))
      (`self.SetMenuVisibility` false :!label _label))))

(event `self.ClickListenerUpgradeText.OnClicked`
  (params (TouchedComponent :type "PrimitiveComponent Object Reference") (ButtonPressed :type "Key Structure"))
  (bind _level (`self.Level`))
  (bind _returnvalue (+ (`self.BaseUpgradePrice`) (* (`self.UpgradePricePerLevel`) (`self.Level`))))
  ;[1 1 1] OnUpgrade/Repair/SellClicked
  (if (`SceneComponent.IsVisible` (`|GetArrayItem` (`SceneComponent.GetParentComponents` TouchedComponent)))
    (if (< _level (`self.MaxLevel`))
      (if (>= (`/Game/Blueprints/CoinsManager.CurrentCoins` (`self.ScoreController`)) _returnvalue)
        (`/Game/Blueprints/CoinsManager.SubstractCoins` (`self.ScoreController`) _returnvalue)
        (set `self.Level` (+ _level 1))
        (set `self.MaxHealthPoints` (+ (`self.MaxHealthPoints`) (`self.HealthLevelIncrement`)))
        (set `self.CurrentHealthPoints` (+ (`self.CurrentHealthPoints`) (`self.HealthLevelIncrement`)))
        (`self.SetLifeText`)
        (set `self.ShotCooldown` (* (`self.ShotCooldown`) (`self.ShotCooldownLevelFactor`)))
        (`MaterialInstanceDynamic.SetVectorParameterValue` (`self.DynamicMaterial`) "DiffuseColor" (`KismetMathLibrary.LinearColorLerp` (`self.StartingColor`) (`self.MaxLevelColor`) (/ (`KismetMathLibrary.Conv_IntToDouble` (`self.Level`)) (`KismetMathLibrary.Conv_IntToDouble` (`self.MaxLevel`)))))
        (`PrimitiveComponent.SetMaterial` (`self.TowerHead`) 0 (`self.DynamicMaterial`))
        (`PrimitiveComponent.SetMaterial` (`self.TowerBody`) 0 (`self.DynamicMaterial`))
        (`PrimitiveComponent.SetMaterial` (`self.ShotSpawn`) 0 (`self.DynamicMaterial`))
        (`PrimitiveComponent.SetMaterial` (`self.Canion`) 0 (`self.DynamicMaterial`))
        (goto _label)))))

(event `self.ClickListenerSellText.OnClicked`
  (params (TouchedComponent :type "PrimitiveComponent Object Reference") (ButtonPressed :type "Key Structure"))
  ;[1 1 1] OnUpgrade/Repair/SellClicked
  (if (`SceneComponent.IsVisible` (`|GetArrayItem` (`SceneComponent.GetParentComponents` TouchedComponent)))
    (`/Game/Blueprints/CoinsManager.AddCoins` (`self.ScoreController`) (+ (`self.SellingPrice`) (* (`self.Level`) (`self.UpgradePricePerLevel`))))
    (`self.Death`)))

(event `self.FullTowerClickListener.OnBeginCursorOver`
  (params (TouchedComponent :type "PrimitiveComponent Object Reference"))
  ;[1 1 1] OnTowerHover
  (`self.SetTowerHoverMaterial`))

(event `self.FullTowerClickListener.OnEndCursorOver`
  (params (TouchedComponent :type "PrimitiveComponent Object Reference"))
  ;[1 1 1] OnTowerHover
  (if (not (`SceneComponent.IsVisible` (`self.RepairText`)))
    (`self.SetTowerNormalMaterial`)))

(event `self.ClickListenerRepairText.OnBeginCursorOver`
  (params (TouchedComponent :type "PrimitiveComponent Object Reference"))
  ;[1 1 1] OnUpgrade/RepairHover
  (`TextRenderComponent.SetWorldSize` (`self.RepairText`) (`self.HoverTextFontSize`)))

(event `self.ClickListenerRepairText.OnEndCursorOver`
  (params (TouchedComponent :type "PrimitiveComponent Object Reference"))
  ;[1 1 1] OnUpgrade/RepairHover
  (`TextRenderComponent.SetWorldSize` (`self.RepairText`) (`self.TextFontSize`)))

(event `self.ClickListenerUpgradeText.OnBeginCursorOver`
  (params (TouchedComponent :type "PrimitiveComponent Object Reference"))
  ;[1 1 1] OnUpgrade/RepairHover
  (`TextRenderComponent.SetWorldSize` (`self.UpgradeText`) (`self.HoverTextFontSize`)))

(event `self.ClickListenerUpgradeText.OnEndCursorOver`
  (params (TouchedComponent :type "PrimitiveComponent Object Reference"))
  ;[1 1 1] OnUpgrade/RepairHover
  (`TextRenderComponent.SetWorldSize` (`self.UpgradeText`) (`self.TextFontSize`)))

(event `self.ClickListenerSellText.OnBeginCursorOver`
  (params (TouchedComponent :type "PrimitiveComponent Object Reference"))
  ;[1 1 1] OnUpgrade/RepairHover
  (`TextRenderComponent.SetWorldSize` (`self.SellText`) (`self.HoverTextFontSize`)))

(event `self.ClickListenerSellText.OnEndCursorOver`
  (params (TouchedComponent :type "PrimitiveComponent Object Reference"))
  ;[1 1 1] OnUpgrade/RepairHover
  (`TextRenderComponent.SetWorldSize` (`self.SellText`) (`self.TextFontSize`)))

(fn `Death`
  (`|SpawnActorFromClass` "/Game/Blueprints/TowerSpawnPoint.TowerSpawnPoint_C" (`KismetMathLibrary.Conv_VectorToTransform` (`self.K2_GetActorLocation` self)) "Undefined" "OverrideRootScale" null (`self.ScoreController`) null)
  (`self.K2_DestroyActor`))

(fn `GetProjectileSpeed`
  (params (TargetLocation :type "Vector Structure"))
  (returns (InitialSpeed :type "Float (double-precision)"))
  (locals (Angle :type "Float (double-precision)" :default 0.0) (InitialHeight :type "Float (double-precision)" :default 0.0) (Distance :type "Float (double-precision)" :default 0.0) (AngleSin :type "Float (double-precision)") (AngleCos :type "Float (double-precision)"))
  (bind _towerhead (`self.TowerHead`))
  (bind _pitch (.pitch (`SceneComponent.K2_GetComponentRotation` _towerhead)))
  (set `local.AngleSin` (`KismetMathLibrary.DegSin` _pitch))
  (set `local.AngleCos` (`KismetMathLibrary.DegCos` _pitch))
  (set `local.InitialHeight` (.z (`SceneComponent.K2_GetComponentLocation` _towerhead)))
  (set `local.Distance` (`KismetMathLibrary.VSize` (- (`SceneComponent.K2_GetComponentLocation` (`self.DefaultSceneRoot`)) TargetLocation)))
  (return (* (`KismetMathLibrary.Sqrt` (/ (* (`KismetMathLibrary.Square` 9.8) (`KismetMathLibrary.Square` (`local.Distance`))) (+ (`local.InitialHeight`) (* (`local.AngleSin`) (/ (`local.Distance`) (`local.AngleCos`)) 2.0 (`KismetMathLibrary.Square` (`local.AngleCos`)))))) 2.0)))

(fn `RecibirDamage`
  (params (DamageAmount :type Integer))
  (bind _output_get (set `self.CurrentHealthPoints` (- (`self.CurrentHealthPoints`) DamageAmount)))
  (if (<= _output_get 0)
    (`self.Death`)
    (else
      (`self.SetLifeText`))))

(fn `SetLifeText`
  (`TextRenderComponent.K2_SetText` (`self.LifeText`) (`KismetTextLibrary.Conv_StringToText` (`KismetStringLibrary.Concat_StrStr` (`KismetStringLibrary.Concat_StrStr` (`KismetStringLibrary.Conv_IntToString` (`self.CurrentHealthPoints`)) "/") (`KismetStringLibrary.Conv_IntToString` (`self.MaxHealthPoints`))))))

(fn `SetMenuVisibility`
  (params (NewVisibility :type Boolean))
  (`SceneComponent.SetVisibility` (`self.RepairText`) NewVisibility false)
  (`SceneComponent.SetVisibility` (`self.UpgradeText`) NewVisibility false)
  (`SceneComponent.SetVisibility` (`self.SellText`) NewVisibility false))

(fn `SetTowerHover`
  (params (Hover :type Boolean))
  (if Hover
    (`self.SetTowerHoverMaterial`)
    (else
      (`self.SetTowerNormalMaterial`))))

(fn `UserConstructionScript`
  (bind _repairtext (`self.RepairText`))
  (set `self.TimeWhenLastShot` (* (`self.ShotCooldown`) -1.0))
  (`self.SetLifeText`)
  (bind _output_get (set `self.TextFontSize` (.z (`TextRenderComponent.GetTextWorldSize` _repairtext))))
  (`TextRenderComponent.SetWorldSize` _repairtext _output_get)
  (bind _returnvalue (`PrimitiveComponent.CreateDynamicMaterialInstance` (`self.TowerBody`) 0 "/Game/Models/BaseMaterial.BaseMaterial"))
  (bind _output_get_2 (set `self.DynamicMaterial` _returnvalue))
  (bind _returnvalue_2 (`MaterialInstanceDynamic.K2_GetVectorParameterValue` _output_get_2 "DiffuseColor"))
  (set `self.StartingColor` _returnvalue_2))