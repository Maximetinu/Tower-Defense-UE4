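; Enemy spawner actor that periodically spawns enemies at the first point of a spline path taken from a referenced scene actor.
; BeginPlay reports a missing spline, measures the path length and finds the camera actor named PlayerCamera.
; Tick calls Spawn at a timed interval, passing each enemy the path, its length, the camera and the spawner.
; DeathThenSpawn spawns another enemy when SpawnWhenDead is set.
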(event `self.ReceiveBeginPlay`
  (bind _path (`self.Path`))
  (if (== (`self.Path`) null)
    (`KismetSystemLibrary.PrintText` "ERROR! Path asignado a EnemySpawner no es un Spline" true true (struct :`R` 0.494792 :`G` 0.006096 :`A` 1.0) 20.0))
  (set `self.SplineLongitude` (`SplineComponent.GetDistanceAlongSplineAtSplinePoint` _path (- (`SplineComponent.GetNumberOfSplinePoints` _path) 1)))
  (bind _outactors (`GameplayStatics.GetAllActorsOfClass` "/Script/Engine.CameraActor"))
  (for _array_element _outactors
    (if (`KismetStringLibrary.EqualEqual_StrStr` (`KismetStringLibrary.Conv_ObjectToString` _array_element) "PlayerCamera")
      (set `self.CameraActor` _array_element))))

(event `self.ReceiveTick`
  (params (DeltaSeconds :type "Float (single-precision)"))
  (if (>= (- (`self.GetGameTimeSinceCreation`) (`self.LastSpawnTime`)) (`self.TimeBetweenSpawns`))
    (set `self.LastSpawnTime` (`self.GetGameTimeSinceCreation`))
    (`self.Spawn`)))

(fn `DeathThenSpawn`
  (if (`self.SpawnWhenDead`)
    (`self.Spawn`)))

(fn `Spawn`
  (`|SpawnActorFromClass` "/Game/Blueprints/Enemy.Enemy_C" (`KismetMathLibrary.Conv_VectorToTransform` (`SplineComponent.GetLocationAtSplinePoint` (`self.Path`) 0 "World")) "Undefined" "OverrideRootScale" null (`self.Path`) (`self.SplineLongitude`) (`self.CameraActor`) self null))

(fn `UserConstructionScript`
  (set `self.Path` (`self.GetComponentByClass` (`self.PathSceneActor`) "/Script/Engine.SplineComponent")))