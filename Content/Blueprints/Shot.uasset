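; Shot is a projectile Blueprint that damages enemies on impact.
; When its static mesh hits a component tagged Enemy, it casts the owner to Enemy, calls RecibirDamage with its Damage value and destroys itself; untagged hits also destroy it.
; The construction script applies the configurable InitialSpeed to the projectile movement and multiplies the actor's uniform scale by Scale.
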(event `self.StaticMeshComponent.OnComponentHit`
  (params (HitComponent :type "PrimitiveComponent Object Reference") (OtherActor :type "Actor Object Reference") (OtherComp :type "PrimitiveComponent Object Reference") (NormalImpulse :type "Vector Structure") (Hit :type "HitResult Structure (by ref)"))
  (if (`ActorComponent.ComponentHasTag` OtherComp "Enemy")
    (bind _asenemy (cast `/Game/Blueprints/Enemy` (`ActorComponent.GetOwner` OtherComp)))
    (`/Game/Blueprints/Enemy.RecibirDamage` _asenemy (`self.Damage`)))
  (`self.K2_DestroyActor`))

(fn `UserConstructionScript`
  (set `ProjectileMovementComponent.InitialSpeed` (`self.InitialSpeed`) (`self.ProjectileMovement`))
  (`self.SetActorScale3D` (`KismetMathLibrary.Conv_DoubleToVector` (* (`self.Scale`) (.x (`SceneComponent.K2_GetComponentScale` (`self.StaticMeshComponent`)))))))