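; MotherBase is a base actor with health points that takes damage through RecibirDamage and quits the game when health reaches zero.
; On Tick it regenerates one point at a timed interval while below maximum.
; A text component shows current and maximum health, turned each frame to face the CameraActor named "PlayerCamera", which is looked up at BeginPlay.
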(event `self.ReceiveBeginPlay`
  (bind _lifetext (`self.LifeText`))
  (set `self.CurrentHealthPoints` (`self.MaxHealthPoints`))
  (bind _outactors (`GameplayStatics.GetAllActorsOfClass` "/Script/Engine.CameraActor"))
  (for _array_element _outactors
    (if (`KismetStringLibrary.EqualEqual_StrStr` (`KismetStringLibrary.Conv_ObjectToString` _array_element) "PlayerCamera")
      (bind _output_get (set `self.CameraActor` _array_element))))
  (bind _output_get_2 (set `self.LookAtCameraRotation` (`KismetMathLibrary.FindLookAtRotation` (`SceneComponent.K2_GetComponentLocation` _lifetext) (`self.K2_GetActorLocation` _output_get))))
  (`SceneComponent.K2_SetWorldRotation` _lifetext _output_get_2 false false)
  (`self.SetLifeText`))

(event `self.ReceiveTick`
  (params (DeltaSeconds :type "Float (single-precision)"))
  (bind _lifetext (`self.LifeText`))
  (`SceneComponent.K2_SetWorldRotation` _lifetext (`KismetMathLibrary.FindLookAtRotation` (`SceneComponent.K2_GetComponentLocation` _lifetext) (`self.K2_GetActorLocation` (`self.CameraActor`))) false false)
  (if (< (`self.CurrentHealthPoints`) (`self.MaxHealthPoints`))
    (if (>= (- (`self.GetGameTimeSinceCreation`) (`self.LastRecover`)) (`self.RecoverOneEachSeconds`))
      (`/Engine/EditorBlueprintResources/StandardMacros.IncrementInt` (`self.CurrentHealthPoints`)
        (:`  `
          (`self.SetLifeText`)
          (set `self.LastRecover` (`self.GetGameTimeSinceCreation`)))))))

(fn `Death`
  (`KismetSystemLibrary.QuitGame` null "Quit"))

(fn `RecibirDamage`
  (params (DamageAmount :type Integer))
  (bind _output_get (set `self.CurrentHealthPoints` (- (`self.CurrentHealthPoints`) DamageAmount)))
  (if (<= _output_get 0)
    (`self.Death`)
    (else
      (`self.SetLifeText`))))

(fn `SetLifeText`
  (`TextRenderComponent.K2_SetText` (`self.LifeText`) (`KismetTextLibrary.Conv_StringToText` (`KismetStringLibrary.Concat_StrStr` (`KismetStringLibrary.Concat_StrStr` (`KismetStringLibrary.Conv_IntToString` (`self.CurrentHealthPoints`)) "/") (`KismetStringLibrary.Conv_IntToString` (`self.MaxHealthPoints`))))))

(fn `UserConstructionScript`
  (`self.SetLifeText`))