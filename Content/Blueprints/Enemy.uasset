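; Enemy that advances along a spline path, facing its direction of travel and showing camera-facing health text.
; Construction scales hit power, speed and max health by level and tints the body material toward a max-level color.
; Overlapping Tower-tagged components knocks it back along the spline and damages the Tower, TowerBomb or MotherBase.
; On death it notifies its spawner, spawns a level-based coin FloatingScore and destroys itself.
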(event `self.ReceiveBeginPlay`
  (set `self.CurrentHealthPoints` (`self.MaxHealthPoints`))
  (`self.SetLifeText`))

(event `self.Body.OnComponentBeginOverlap`
  (params (OverlappedComponent :type "PrimitiveComponent Object Reference") (OtherActor :type "Actor Object Reference") (OtherComp :type "PrimitiveComponent Object Reference") (OtherBodyIndex :type Integer) (bFromSweep :type Boolean) (SweepResult :type "HitResult Structure (by ref)"))
  (if (`ActorComponent.ComponentHasTag` OtherComp "Tower")
    (set `self.CurrentSplineDistance` (- (`self.CurrentSplineDistance`) (`self.HitBounce`)))
    (bind _astower (cast `/Game/Blueprints/Tower` OtherActor)
      (:`then`
        (`/Game/Blueprints/Tower.RecibirDamage` _astower (`self.HitPower`)))
      (:`CastFailed`
        (bind _astower_bomb (cast `/Game/Blueprints/TowerBomb` OtherActor)
          (:`then`
            (`/Game/Blueprints/TowerBomb.RecibirDamage` _astower_bomb (`self.HitPower`)))
          (:`CastFailed`
            (bind _asmother_base (cast `/Game/Blueprints/MotherBase` OtherActor))
            (`/Game/Blueprints/MotherBase.RecibirDamage` _asmother_base (`self.HitPower`))))))))

(event `self.ReceiveTick`
  (params (DeltaSeconds :type "Float (single-precision)"))
  (bind _defaultsceneroot (`self.DefaultSceneRoot`))
  (bind _maxsplinedistance (`self.MaxSplineDistance`))
  (bind _lifetext (`self.LifeText`))
  (bind _output_get (set `self.CurrentSplineDistance` (+ (* DeltaSeconds (`self.Speed`)) (`self.CurrentSplineDistance`))))
  (if (> _output_get _maxsplinedistance)
    (set `self.CurrentSplineDistance` _maxsplinedistance))
  (bind _returnvalue (`SplineComponent.GetLocationAtDistanceAlongSpline` (`self.EnemyPath`) _output_get "World"))
  (`SceneComponent.K2_SetWorldLocationAndRotation` _defaultsceneroot _returnvalue (`KismetMathLibrary.FindLookAtRotation` (`SceneComponent.K2_GetComponentLocation` _defaultsceneroot) _returnvalue) false false)
  (`SceneComponent.K2_SetWorldRotation` _lifetext (`KismetMathLibrary.FindLookAtRotation` (`SceneComponent.K2_GetComponentLocation` _lifetext) (`self.K2_GetActorLocation` (`self.CameraActor`))) false false)
  (`self.SetLifeText`))

(fn `Death`
  (`/Game/Blueprints/EnemySpawner.DeathThenSpawn` (`self.EnemySpawner`))
  (`|SpawnActorFromClass` "/Game/Blueprints/FloatingScore.FloatingScore_C" (`KismetMathLibrary.Conv_VectorToTransform` (`KismetMathLibrary.MakeVector` (.x (`SceneComponent.K2_GetComponentLocation` (`self.LifeText`))) (.y (`SceneComponent.K2_GetComponentLocation` (`self.LifeText`))) (- (.z (`SceneComponent.K2_GetComponentLocation` (`self.LifeText`))) 75.0))) "Undefined" "OverrideRootScale" null (`self.CameraActor`) (* (+ (`self.Level`) 1) (`self.CoinsPerLevel`)) null)
  (`self.K2_DestroyActor`))

(fn `RecibirDamage`
  (params (DamageAmount :type Integer))
  (bind _output_get (set `self.CurrentHealthPoints` (- (`self.CurrentHealthPoints`) DamageAmount)))
  (if (<= _output_get 0)
    (`self.Death`)
    (else
      (`self.SetLifeText`))))

(fn `SetLifeText`
  (`TextRenderComponent.K2_SetText` (`self.LifeText`) (`KismetTextLibrary.Conv_StringToText` (`KismetStringLibrary.Concat_StrStr` (`KismetStringLibrary.Concat_StrStr` (`KismetStringLibrary.Conv_IntToString` (`self.CurrentHealthPoints`)) "/") (`KismetStringLibrary.Conv_IntToString` (`self.MaxHealthPoints`))))))

(fn `UserConstructionScript`
  (set `self.HitPower` (+ (`self.HitPower`) (* (`self.DamageIncrementPerLevel`) (`self.Level`))))
  (set `self.Speed` (+ (`self.Speed`) (* (`self.Level`) (`self.SpeedIncrementPerLevel`))))
  (set `self.MaxHealthPoints` (+ (`self.MaxHealthPoints`) (* (`self.HealthIncrementPerLevel`) (`self.Level`))))
  (bind _returnvalue (`PrimitiveComponent.CreateDynamicMaterialInstance` (`self.Body`) 0 "/Game/Models/BaseMaterial.BaseMaterial"))
  (bind _returnvalue_2 (`MaterialInstanceDynamic.K2_GetVectorParameterValue` _returnvalue "DiffuseColor"))
  (set `self.StartingColor` _returnvalue_2)
  (`MaterialInstanceDynamic.SetVectorParameterValue` _returnvalue "DiffuseColor" (`KismetMathLibrary.LinearColorLerp` (`self.StartingColor`) (`self.MaxLevelColor`) (/ (`KismetMathLibrary.Conv_IntToDouble` (`self.Level`)) (`KismetMathLibrary.Conv_IntToDouble` (`self.MaxLevel`))))))