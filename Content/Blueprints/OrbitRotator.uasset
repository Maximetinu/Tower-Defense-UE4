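; OrbitRotator is a component that spins its owning actor around yaw while rocking it in roll and pitch.
; Each Tick adds speed-scaled delta time to the current yaw and sets roll and pitch absolutely from magnitude-scaled sine values, computed the previous frame.
; Both incline speeds advance one shared phase, wrapped at two pi, so both axes oscillate at the combined rate with only a small per-frame offset.
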(event `self.ReceiveTick`
  (params (DeltaSeconds :type "Float (single-precision)"))
  (bind _returnvalue (`self.GetOwner`))
  (bind _returnvalue_2 (* (`KismetMathLibrary.GetPI`) 2.0))
  (bind _returnvalue_3 (* (`KismetMathLibrary.GetPI`) 2.0))
  (`Actor.K2_SetActorRotation` _returnvalue (`KismetMathLibrary.MakeRotator` (+ (* (stale _output_get_2) (`self.XMagnitude`)) 0.0) (+ (* (stale _output_get_4) (`self.YMagnitude`)) 0.0) (+ (.yaw (`Actor.K2_GetActorRotation` _returnvalue)) (* DeltaSeconds (`self.RotationSpeed`)))) false)
  (set `self.Sin` (+ (`self.Sin`) (* DeltaSeconds (`self.InclineXSpeed`))))
  (if (>= (`self.Sin`) _returnvalue_2)
    (bind _output_get (set `self.Sin` (- (`self.Sin`) _returnvalue_2))))
  (bind _output_get_2 (set `self.CurrentXIncline` (`KismetMathLibrary.Sin` _output_get)))
  (set `self.Sin` (+ (`self.Sin`) (* DeltaSeconds (`self.InclineYSpeed`))))
  (if (>= (`self.Sin`) _returnvalue_3)
    (bind _output_get_3 (set `self.Sin` (- (`self.Sin`) _returnvalue_3))))
  (bind _output_get_4 (set `self.CurrentYIncline` (`KismetMathLibrary.Sin` _output_get_3))))