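; Clickable tower build spot that lets the player buy a normal or bomb tower with coins.
; Clicking the base toggles two text options, which resize on hover through their click listeners.
; Clicking a visible, affordable option spawns that tower with the ScoreController, subtracts TowerPrice and destroys the spot.
; BeginPlay finds the camera actor named PlayerCamera, and Tick keeps both labels rotated toward it.
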(event `self.ReceiveBeginPlay`
  (bind _bombtowertext (`self.BombTowerText`))
  (bind _normaltowertext (`self.NormalTowerText`))
  (bind _outactors (`GameplayStatics.GetAllActorsOfClass` "/Script/Engine.CameraActor"))
  (for _array_element _outactors
    (if (`KismetStringLibrary.EqualEqual_StrStr` (`KismetStringLibrary.Conv_ObjectToString` _array_element) "PlayerCamera")
      (bind _output_get (set `self.CameraActor` _array_element))
      (bind _returnvalue (`self.K2_GetActorLocation` _output_get))
      (`SceneComponent.K2_SetWorldRotation` _bombtowertext (`KismetMathLibrary.FindLookAtRotation` (`SceneComponent.K2_GetComponentLocation` _bombtowertext) _returnvalue) false false)
      (`SceneComponent.K2_SetWorldRotation` _normaltowertext (`KismetMathLibrary.FindLookAtRotation` (`SceneComponent.K2_GetComponentLocation` _normaltowertext) _returnvalue) false false))))

(event `self.Base.OnClicked`
  (params (TouchedComponent :type "PrimitiveComponent Object Reference") (ButtonPressed :type "Key Structure"))
  (bind _bombtowertext (`self.BombTowerText`))
  (bind _normaltowertext (`self.NormalTowerText`))
  (`SceneComponent.SetVisibility` _bombtowertext (!= (`SceneComponent.IsVisible` _bombtowertext) true) false)
  (`SceneComponent.SetVisibility` _normaltowertext (!= (`SceneComponent.IsVisible` _normaltowertext) true) false))

(event `self.NormalTowerClickListener.OnBeginCursorOver`
  (params (TouchedComponent :type "PrimitiveComponent Object Reference"))
  (`TextRenderComponent.SetWorldSize` (`self.NormalTowerText`) (`self.HoverTextFontSize`)))

(event `self.NormalTowerClickListener.OnEndCursorOver`
  (params (TouchedComponent :type "PrimitiveComponent Object Reference"))
  (`TextRenderComponent.SetWorldSize` (`self.NormalTowerText`) (`self.TextFontSize`)))

(event `self.BombTowerClickListener.OnBeginCursorOver`
  (params (TouchedComponent :type "PrimitiveComponent Object Reference"))
  (`TextRenderComponent.SetWorldSize` (`self.BombTowerText`) (`self.HoverTextFontSize`)))

(event `self.BombTowerClickListener.OnEndCursorOver`
  (params (TouchedComponent :type "PrimitiveComponent Object Reference"))
  (`TextRenderComponent.SetWorldSize` (`self.BombTowerText`) (`self.TextFontSize`)))

(event `self.ReceiveTick`
  (params (DeltaSeconds :type "Float (single-precision)"))
  (`SceneComponent.K2_SetWorldRotation` (`self.NormalTowerText`) (`KismetMathLibrary.FindLookAtRotation` (`SceneComponent.K2_GetComponentLocation` (`self.DefaultSceneRoot`)) (`self.K2_GetActorLocation` (`self.CameraActor`))) false false)
  (`SceneComponent.K2_SetWorldRotation` (`self.BombTowerText`) (`KismetMathLibrary.FindLookAtRotation` (`SceneComponent.K2_GetComponentLocation` (`self.DefaultSceneRoot`)) (`self.K2_GetActorLocation` (`self.CameraActor`))) false false))

(event `self.NormalTowerClickListener.OnClicked`
  (params (TouchedComponent :type "PrimitiveComponent Object Reference") (ButtonPressed :type "Key Structure"))
  (bind _towerprice (`self.TowerPrice`))
  (if (`SceneComponent.IsVisible` (`|GetArrayItem` (`SceneComponent.GetParentComponents` TouchedComponent)))
    (if (>= (`/Game/Blueprints/CoinsManager.CurrentCoins` (`self.ScoreController`)) _towerprice)
      (`|SpawnActorFromClass` "/Game/Blueprints/Tower.Tower_C" (`KismetMathLibrary.Conv_VectorToTransform` (`SceneComponent.K2_GetComponentLocation` (`self.DefaultSceneRoot`))) "Undefined" "OverrideRootScale" null (`self.ScoreController`) null)
      (`/Game/Blueprints/CoinsManager.SubstractCoins` (`self.ScoreController`) _towerprice)
      (`self.K2_DestroyActor` self))))

(event `self.BombTowerClickListener.OnClicked`
  (params (TouchedComponent :type "PrimitiveComponent Object Reference") (ButtonPressed :type "Key Structure"))
  (bind _towerprice (`self.TowerPrice`))
  (if (`SceneComponent.IsVisible` (`|GetArrayItem` (`SceneComponent.GetParentComponents` TouchedComponent)))
    (if (>= (`/Game/Blueprints/CoinsManager.CurrentCoins` (`self.ScoreController`)) _towerprice)
      (`|SpawnActorFromClass` "/Game/Blueprints/TowerBomb.TowerBomb_C" (`KismetMathLibrary.Conv_VectorToTransform` (`SceneComponent.K2_GetComponentLocation` (`self.DefaultSceneRoot`))) "Undefined" "OverrideRootScale" null (`self.ScoreController`) null)
      (`/Game/Blueprints/CoinsManager.SubstractCoins` (`self.ScoreController`) _towerprice)
      (`self.K2_DestroyActor` self))))

(fn `UserConstructionScript`)