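; FakeEnemy is a placeholder enemy actor that tracks health and shows it as current/max text on LifeText.
; RecibirDamage subtracts damage, then either refreshes the text or calls Death when health reaches zero or below.
; Death destroys the actor and notifies its EnemySpawner through DeathThenSpawn.
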(fn `Death`
  (`self.K2_DestroyActor`)
  (`/Game/Blueprints/EnemySpawner.DeathThenSpawn` (`self.EnemySpawner`)))

(fn `RecibirDamage`
  (params (DamageAmount :type Integer))
  (bind _output_get (set `self.CurrentHealthPoints` (- (`self.CurrentHealthPoints`) DamageAmount)))
  (if (<= _output_get 0)
    (`self.Death`)
    (else
      (`self.SetLifeText`))))

(fn `SetLifeText`
  (`TextRenderComponent.K2_SetText` (`self.LifeText`) (`KismetTextLibrary.Conv_StringToText` (`KismetStringLibrary.Concat_StrStr` (`KismetStringLibrary.Concat_StrStr` (`KismetStringLibrary.Conv_IntToString` (`self.CurrentHealthPoints`)) "/") (`KismetStringLibrary.Conv_IntToString` (`self.MaxHealthPoints`))))))

(fn `UserConstructionScript`)