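; Tower defense turret actor that aims at and shoots enemies within its range.
; The ShootingRadius overlap events add actors tagged Enemy to PotentialTargets and remove them when they leave.
; Each tick it snaps TowerHead toward the first target in the list and spawns a Shot at ShotSpawn whenever ShotCooldown has elapsed.
; The construction script backdates TimeWhenLastShot by one cooldown so the first shot needs no wait.
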(event `self.ShootingRadius.OnComponentEndOverlap`
  (params (OverlappedComponent :type "PrimitiveComponent Object Reference") (OtherActor :type "Actor Object Reference") (OtherComp :type "PrimitiveComponent Object Reference") (OtherBodyIndex :type Integer))
  (`KismetArrayLibrary.Array_RemoveItem` (`self.PotentialTargets`) OtherActor))

(event `self.ShootingRadius.OnComponentBeginOverlap`
  (params (OverlappedComponent :type "PrimitiveComponent Object Reference") (OtherActor :type "Actor Object Reference") (OtherComp :type "PrimitiveComponent Object Reference") (OtherBodyIndex :type Integer) (bFromSweep :type Boolean) (SweepResult :type "HitResult Structure (by ref)"))
  (if (`self.ActorHasTag` OtherActor "Enemy")
    (`KismetArrayLibrary.Array_Add` (`self.PotentialTargets`) OtherActor)))

(event `self.ReceiveTick`
  (params (DeltaSeconds :type "Float (single-precision)"))
  (bind _towerhead (`self.TowerHead`))
  (bind _shotspawn (`self.ShotSpawn`))
  (if (> (`KismetArrayLibrary.Array_Length` (`self.PotentialTargets`)) 0)
    (`SceneComponent.K2_SetWorldRotation` _towerhead (`KismetMathLibrary.FindLookAtRotation` (`SceneComponent.K2_GetComponentLocation` _towerhead) (`self.K2_GetActorLocation` (`|GetArrayItem` (`self.PotentialTargets`)))) false false)
    (if (>= (- (`self.GetGameTimeSinceCreation`) (`self.TimeWhenLastShot`)) (`self.ShotCooldown`))
      (`|SpawnActorFromClass` "/Game/Blueprints/Shot.Shot_C" (`KismetMathLibrary.MakeTransform` (`SceneComponent.K2_GetComponentLocation` _shotspawn) (`SceneComponent.K2_GetComponentRotation` _shotspawn)) "AlwaysSpawn" "OverrideRootScale" null null)
      (set `self.TimeWhenLastShot` (`self.GetGameTimeSinceCreation`)))))

(fn `UserConstructionScript`
  (set `self.TimeWhenLastShot` (* (`self.ShotCooldown`) -1.0)))