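; FloatingScore is an actor that shows a coin gain as floating text, formatted with a plus sign and a dollar suffix.
; On BeginPlay it sets the text from Coins and turns the TextRender toward the Camera actor once.
; Each Tick it moves the root upward with constant acceleration, using InitialSpeed as the running velocity, and destroys itself at a fixed world height.
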(event `self.ReceiveBeginPlay`
  (bind _textrender (`self.TextRender`))
  (`SceneComponent.K2_SetWorldRotation` _textrender (`KismetMathLibrary.FindLookAtRotation` (`SceneComponent.K2_GetComponentLocation` _textrender) (`self.K2_GetActorLocation` (`self.Camera`))) false false)
  (`TextRenderComponent.K2_SetText` (`self.TextRender`) (`KismetTextLibrary.Conv_StringToText` (`KismetStringLibrary.Concat_StrStr` "+" (`KismetStringLibrary.Conv_IntToString` (`self.Coins`)) "$"))))

(event `self.ReceiveTick`
  (params (DeltaSeconds :type "Float (single-precision)"))
  (bind _defaultsceneroot (`self.DefaultSceneRoot`))
  (`SceneComponent.K2_SetWorldLocation` _defaultsceneroot (+ (`SceneComponent.K2_GetComponentLocation` _defaultsceneroot) (`KismetMathLibrary.MakeVector` 0.0 0.0 (* (`self.InitialSpeed`) DeltaSeconds))) false false)
  (set `self.InitialSpeed` (+ (* (`self.Acceleration`) DeltaSeconds) (`self.InitialSpeed`)))
  (if (>= (.z (`SceneComponent.K2_GetComponentLocation` (`self.DefaultSceneRoot`))) 4000.0)
    (`self.K2_DestroyActor`)))

(fn `UserConstructionScript`)